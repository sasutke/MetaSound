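; BP_Minigun is a minigun turret prototype Blueprint that spins a static mesh and animates its material.
; On BeginPlay it starts the Rotate timeline, whose value scales a per-tick world yaw rotation of StaticMesh1.
; It also creates a dynamic material instance, then after a short delay a second timeline drives that material's scalar parameter.
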(event `self.ReceiveTick`
  (params (DeltaSeconds :type "Float (single-precision)"))
  (`SceneComponent.K2_AddWorldRotation` (`self.StaticMesh1`) (`KismetMathLibrary.RLerp` (struct) (struct :`Pitch` 30.0) (stale `self.ReceiveBeginPlay` _newtrack_0)) false false))

(event `self.ReceiveBeginPlay`
  (`|ExecutionSequence`
    (:`then_0`
      (bind (_direction _newtrack_0) (`Timeline|Rotate`)))
    (:`then_1`
      (bind _returnvalue (`PrimitiveComponent.CreateDynamicMaterialInstance` (`self.StaticMesh1`) 0 "/Game/DX3/P_TA/HW_Proto/Material/MI_Minigun_turret_BaseColor_Mat.MI_Minigun_turret_BaseColor_Mat" "None"))
      (`KismetSystemLibrary.Delay` 3.0)
      (bind (_direction_2 _newtrack_0_2) (`Timeline|Timeline`)
        (:`Update`
          (`MaterialInstanceDynamic.SetScalarParameterValue` _returnvalue "Param" _newtrack_0_2))))))

(fn `UserConstructionScript`)